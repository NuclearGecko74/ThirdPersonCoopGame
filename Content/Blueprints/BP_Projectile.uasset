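; BP_Projectile is a timed explosive projectile that detonates two seconds after it begins play.
; Its Explode event spawns a scaled-up explosion particle and applies full radial damage within DamageRadius, credited to the instigator's controller.
; It then destroys the actor, draws a debug sphere of the blast radius and plays a grenade-launcher sound at world origin rather than the blast location.
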(event Custom|Explode
  (bind _returnvalue (Transformation|GetActorLocation))
  (Effects|SpawnEmitteratLocation "/Game/WeaponEffects/Explosion/P_Explosion.P_Explosion" _returnvalue "0, 0, 0" "2.000000,2.000000,2.000000" false)
  (Game|Damage|ApplyRadialDamage 1e+02 _returnvalue (Variables|Default|GetDamageRadius) 0 0 self (Game|GetInstigatorController) true "ECC_Visibility")
  (Actor|DestroyActor)
  (Rendering|Debug|DrawDebugSphere _returnvalue (Variables|Default|GetDamageRadius) 12 "(R=0.740212,G=1.000000,B=0.000000,A=1.000000)" 1.0 1.0)
  (Audio|PlaySoundatLocation "/Game/MilitaryWeapSilver/Sound/GrenadeLauncher/Cues/GrenadeLauncher_Explosion_Cue.GrenadeLauncher_Explosion_Cue" "0, 0, 0" "0, 0, 0" 1.0 1.0 0.0 0 0 0))

(event EventBeginPlay
  (Utilities|FlowControl|Delay 2.0)
  (CallFunction|Explode))

(fn ConstructionScript)